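; Melee enemy character with a health bar, montage attacks and ragdoll death.
; Damage lowers health in BPCStats, halts walking during the hit-react montage and sets the blackboard phase 2 flag at half health or below.
; Sword trace events run a looping sphere-trace timer with DoOnce-throttled damage, using GetSwordTracePoints for bosses and scene components otherwise.
; A separate single-point sphere trace deals fixed damage.
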(event `self.ReceiveBeginPlay`
  (bind _aswb_enemy_health (cast `/Game/UI/WB_EnemyHealth` (`WidgetComponent.GetWidget` (`self.Widget`))))
  (`/Game/Blueprints/BPC_Stats.Set Health Progress Bar` (`self.BPC_Stats`) (`/Game/UI/WB_EnemyHealth.HealthBar` _aswb_enemy_health)))

(event `self.ReceiveAnyDamage`
  (params (Damage :type "Float (single-precision)") (DamageType :type "DamageType Object Reference") (InstigatedBy :type "Controller Object Reference") (DamageCauser :type "Actor Object Reference"))
  (bind _bpc_stats (`self.BPC_Stats`))
  (bind _charactermovement (`self.CharacterMovement`))
  ; Damage
  (`/Game/Blueprints/BPC_Stats.Increase Value` (`self.BPC_Stats`) "NewEnumerator0" (* Damage -1.0))
  (`|PlayMontage` (`self.Mesh`) (`self.hitReactMontage`)
    (:`then`
      (set `CharacterMovementComponent.MaxWalkSpeed` 0.0 _charactermovement))
    (:`OnCompleted`
      (set `CharacterMovementComponent.MaxWalkSpeed` 300.0 _charactermovement :!label _label))
    (:`OnInterrupted`
      (goto _label)))
  ; Change to Phase 2
  (if (> (`/Game/Blueprints/BPC_Stats.Health` _bpc_stats) (/ (`/Game/Blueprints/BPC_Stats.MaxHealth` _bpc_stats) 2.0))
    (`BlackboardComponent.SetValueAsBool` (`AIBlueprintHelperLibrary.GetBlackboard` null) "phase2?" false)
    (else
      (`BlackboardComponent.SetValueAsBool` (`AIBlueprintHelperLibrary.GetBlackboard` null) "phase2?" true))))

(event `/Game/Blueprints/BPI_Damage.End Sword Trace`
  ; Sword Traces
  (if (`KismetSystemLibrary.K2_IsValidTimerHandle` (stale `/Game/Blueprints/BPI_Damage.Begin Sword Trace` _returnvalue))
    (`KismetSystemLibrary.K2_ClearAndInvalidateTimerHandle` (stale `/Game/Blueprints/BPI_Damage.Begin Sword Trace` _returnvalue))))

(event `/Game/Blueprints/BPI_Damage.Begin Sword Trace`
  ; Sword Traces
  (bind _returnvalue (`KismetSystemLibrary.K2_SetTimerDelegate` (delegate `Damage Trace`) 0.01 true)))

(event `Damage Trace`
  ; Sword Traces
  (if (not (`self.isDead?`))
    (bind (_start _end) (`self.GetSwordTracePoints`))
    (bind (_outhit _returnvalue) (`KismetSystemLibrary.SphereTraceSingleForObjects` :`Start` (`KismetMathLibrary.SelectVector` _start (`SceneComponent.K2_GetComponentLocation` (`self.Start Sword Trace Pos`)) (`self.isBoss?`)) :`End` (`KismetMathLibrary.SelectVector` _end (`SceneComponent.K2_GetComponentLocation` (`self.End Sword Trace Pos`)) (`self.isBoss?`)) :`Radius` (`self.swordAttackRadius`) :`ObjectTypes` (`|MakeArray` "ObjectTypeQuery3" :!type "EObjectTypeQuery Enum") :`DrawDebugType` "ForOneFrame"))
    (if _returnvalue
      (`/Engine/EditorBlueprintResources/StandardMacros.DoOnce` false :!label _label_2
        (:`Completed`
          (`GameplayStatics.ApplyDamage` (`.HitActor` (`GameplayStatics.BreakHitResult` _outhit)) (`self.Sword Damage`))
          (`KismetSystemLibrary.Delay` 0.3)
          (goto _label_2 :!via `Reset`))))))

(event `/Game/Blueprints/BPI_Damage.Die`
  (`CharacterMovementComponent.DisableMovement` (`self.CharacterMovement`))
  (`PrimitiveComponent.SetSimulatePhysics` (`self.Mesh`) true)
  (set `self.isDead?` true))

(event `/Game/Blueprints/BPI_Damage.Point Damage Trace`
  (bind _returnvalue (`SceneComponent.K2_GetComponentLocation` (`self.Point Trace Pos`)))
  (bind (_outhit _returnvalue_2) (`KismetSystemLibrary.SphereTraceSingleForObjects` :`Start` _returnvalue :`End` _returnvalue :`Radius` (`self.pointAttackRadius`) :`ObjectTypes` (`|MakeArray` "ObjectTypeQuery3" :!type "EObjectTypeQuery Enum") :`DrawDebugType` "ForDuration" :`DrawTime` 1.0))
  (if _returnvalue_2
    (`GameplayStatics.ApplyDamage` (`.HitActor` (`GameplayStatics.BreakHitResult` _outhit)) 10.0)))

(fn `BigAttack`
  (returns (Duration :type "Float (double-precision)"))
  (bind _returnvalue (`self.PlayAnimMontage` (`self.bigAttackMontage`)))
  (return _returnvalue))

(fn `ComboAttack`
  (returns (Duration :type "Float (double-precision)"))
  (bind _returnvalue (`self.PlayAnimMontage` (`self.comboAttackMontage`)))
  (return _returnvalue))

(fn `GetSwordTracePoints`
  (returns (Start :type "Vector Structure") (End :type "Vector Structure"))
  (bind _returnvalue (`self.K2_GetActorLocation`))
  (return _returnvalue _returnvalue))

(fn `Sword Attack`
  (returns (Duration :type "Float (double-precision)"))
  (bind _returnvalue (`self.PlayAnimMontage` (`self.swordAttackMontage`)))
  (return _returnvalue))

(fn `UserConstructionScript`)